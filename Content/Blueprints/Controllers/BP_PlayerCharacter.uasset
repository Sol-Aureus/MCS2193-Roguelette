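; Player character for a betting game with a ball shop, holding money, bets, owned balls and round progress.
; It creates money, betting, shop and loss widgets, and a level-sequence camera move swaps the betting slider with the shop.
; Bets trigger spins; results pay out after a retriggerable delay, and every three spins either raise the money requirement or show the loss screen.
; Temporary UI setup and debug keys remain.
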(event `Key|E`
  (params (Key :type "Key Structure"))
  ; Debug keys
  (:`Pressed`
    (bind _output_get (set `self.CurrentMoney` (+ (`self.CurrentMoney`) 15)))
    (`self.Event_UpdateUI` _output_get)))

(event `self.ReceiveBeginPlay`
  ; Temporary set up for the ui. Will figure out where to put this later
  (bind _returnvalue (`|CreateWidget` "/Game/Widgets/UI_MoneyDisplay.UI_MoneyDisplay_C"))
  (bind _output_get (set `self.MoneyText` _returnvalue))
  (`UserWidget.AddToViewport` _output_get 0)
  (`/Game/Widgets/UI_MoneyDisplay.UpdateMoney` (`self.MoneyText`) (`self.CurrentMoney`))
  (bind _returnvalue_2 (`|CreateWidget` "/Game/Widgets/UI_BettingSlider.UI_BettingSlider_C"))
  (bind _output_get_2 (set `self.BettingSlider` _returnvalue_2))
  (`UserWidget.AddToViewport` _output_get_2 0)
  (set `PlayerController.bShowMouseCursor` true (`GameplayStatics.GetPlayerController` 0))
  (`/Game/Widgets/UI_BettingSlider.UpdateTotalMoney` (`self.BettingSlider`) (`self.CurrentMoney`))
  (bind _returnvalue_3 (`|CreateWidget` "/Game/Widgets/UI_ShopDisplay.UI_ShopDisplay_C"))
  (set `self.ShopDisplay` _returnvalue_3)
  (bind _returnvalue_4 (`|GenericCreateObject` "/Game/Widgets/UI_LossScreen.UI_LossScreen_C"))
  (set `self.LoseScreen` _returnvalue_4))

(event `Key|R`
  (params (Key :type "Key Structure"))
  ; Debug keys
  (:`Pressed`
    (bind _output_get (set `self.CurrentMoney` (- (`self.CurrentMoney`) 15)))
    (`self.Event_UpdateUI` _output_get)))

(event `Key|A`
  (params (Key :type "Key Structure"))
  ; Debug keys
  (:`Pressed`
    (`self.Event_MoveCamera`)))

(event `Event_UpdateUI`
  (params (Ammount :type Integer))
  ;[0.6609 0.7304 0.2522 0.5] Event to update all ui money values
  (`/Game/Widgets/UI_MoneyDisplay.UpdateMoney` (`self.MoneyText`) Ammount)
  (`/Game/Widgets/UI_BettingSlider.UpdateTotalMoney` (`self.BettingSlider`) Ammount))

(event `Event_MoveCamera`
  ;[0.5061 0.7078 0.353 0.5] Camera Movement
  (bind _outactor (`LevelSequencePlayer.CreateLevelSequencePlayer` "/Game/Sequences/LS_MoveCamera.LS_MoveCamera"))
  (if (`self.CameraMoved`)
    (bind _sequenceplayer (`LevelSequenceActor.SequencePlayer` _outactor))
    (`MovieSceneSequencePlayer.PlayReverse` _sequenceplayer)
    (set `self.CameraMoved` false)
    (`UserWidget.AddToViewport` (`self.BettingSlider`) 0)
    (`Widget.RemoveFromParent` (`self.ShopDisplay`))
    (else
      (`MovieSceneSequencePlayer.Play` _sequenceplayer)
      (set `self.CameraMoved` true)
      (`Widget.RemoveFromParent` (`self.BettingSlider`))
      (`UserWidget.AddToViewport` (`self.ShopDisplay`) 0))))

(event `Event_ItemBuy`
  (params (ItemID :type Integer))
  ;[0.7635 0.15 0.15 0.5] Reciving the input to buy an item
  (switch `int` ItemID
    (:`0`
      ;[0.15 0.9026 0.15 0.5] Checking if the player has enough money
      (if (>= (`self.CurrentMoney`) (`self.BouleCost`))
        ;[0.15 0.15 0.8887 0.5] Buying the item and adding it to the array
        (bind _output_get (set `self.CurrentMoney` (- (`self.CurrentMoney`) (`self.BouleCost`))))
        (`self.Event_UpdateUI` _output_get)
        (`KismetArrayLibrary.Array_Add` (`self.BallArray`) ItemID :!label _label)
        ; Printing the current array of balls
        (for (_array_element _array_index) (`self.BallArray`)
          (`KismetSystemLibrary.PrintString` (`KismetStringLibrary.Concat_StrStr` "Value: " (`KismetStringLibrary.Conv_IntToString` _array_element) " Index: " (`KismetStringLibrary.Conv_IntToString` _array_index))))))
    (:`1`
      (if (>= (`self.CurrentMoney`) (`self.GoldCost`))
        (bind _output_get_2 (set `self.CurrentMoney` (- (`self.CurrentMoney`) (`self.GoldCost`))))
        (`self.Event_UpdateUI` _output_get_2)
        (goto _label)))
    (:`2`
      (if (>= (`self.CurrentMoney`) (`self.BlackRedCost`))
        (bind _output_get_3 (set `self.CurrentMoney` (- (`self.CurrentMoney`) (`self.BlackRedCost`))))
        (`self.Event_UpdateUI` _output_get_3)
        (goto _label)))
    (:`3`
      (if (>= (`self.CurrentMoney`) (`self.BlackRedCost`))
        (bind _output_get_4 (set `self.CurrentMoney` (- (`self.CurrentMoney`) (`self.BlackRedCost`))))
        (`self.Event_UpdateUI` _output_get_4)
        (goto _label)))
    (:`4`
      (if (>= (`self.CurrentMoney`) (`self.GreenCost`))
        (bind _output_get_5 (set `self.CurrentMoney` (- (`self.CurrentMoney`) (`self.GreenCost`))))
        (`self.Event_UpdateUI` _output_get_5)
        (goto _label)))))

(event `Event_Bet`
  (params (Ammount :type Integer) (Color :type "Material Object Reference"))
  ;[0.9043 0.5217 0.4348 0.5] Gets the bet and spins
  (set `self.BetAmmount` Ammount)
  (set `self.BetColor` Color)
  (`/Engine/EditorBlueprintResources/StandardMacros.IncrementInt` (`self.Spins`)
    (:`  `
      (`self.Event_Spin`)
      (bind _output_get (set `self.CurrentMoney` (- (`self.CurrentMoney`) (`self.BetAmmount`))))
      (`self.Event_UpdateUI` _output_get)
      (set `self.Bet` true))))

(event `Event_CallBet`
  (params (Won :type Boolean) (Multi :type "Float (double-precision)"))
  (bind _betammount (`self.BetAmmount`))
  ;[0.3461 0.2904 0.6661 0.5] Determine how much is won from the bet
  (if Won
    (if (`self.Bet`)
      (set `self.TotalWonBet` _betammount))
    (set `self.TotalWonBet` (+ (* Multi _betammount) (`self.TotalWonBet`))))
  (`KismetSystemLibrary.RetriggerableDelay` 4.0)
  (bind _output_get (set `self.CurrentMoney` (+ (`self.CurrentMoney`) (`self.TotalWonBet`))))
  ;[0.313 0.8522 0.6957 0.5] Advances the round and checks if the player has enough money when the 3 spins concludes
  (`self.Event_UpdateUI` _output_get)
  (`self.Event_MoveCamera`)
  (set `self.TotalWonBet` 0)
  (if (>= (`self.Spins`) 3)
    (if (>= (`self.CurrentMoney`) (`self.RequiredMoney`))
      (`/Engine/EditorBlueprintResources/StandardMacros.IncrementInt` (`self.Rounds`)
        (:`  `
          (set `self.RequiredMoney` (* (`self.RequiredMoney`) 1.5))
          (set `self.Spins` 0)))
      (else
        (`UserWidget.AddToViewport` (`self.LoseScreen`) 0)))))

(event `Event_Spin`)

(fn `GetBet`
  (returns (Bet :type Integer))
  (return (`self.BetAmmount`)))

(fn `GetBetColor`
  (returns (Color :type "Material Object Reference"))
  (return (`self.BetColor`)))

(fn `GetLastBall`
  (returns (Value :type Integer))
  (bind _ballarray (`self.BallArray`))
  (bind _returnvalue (`KismetArrayLibrary.Array_LastIndex` _ballarray))
  (`KismetArrayLibrary.Array_Remove` _ballarray _returnvalue)
  (return (`|GetArrayItem` _ballarray _returnvalue)))

(fn `GetRequiredMoney`
  (returns (Money :type Integer))
  (return (`self.RequiredMoney`)))

(fn `GetRounds`
  (returns (Rounds :type Integer))
  (return (`self.Rounds`)))

(fn `GetSpins`
  (returns (Spins :type Integer))
  (return (`self.Spins`)))

(fn `UserConstructionScript`)