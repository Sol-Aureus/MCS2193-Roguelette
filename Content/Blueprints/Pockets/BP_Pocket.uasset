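; BP_Pocket is a pocket actor that reacts to overlapping Boule, Gold and Paint actors, identified by their first tag.
; Gold raises the base, black and green values by GoldIncrease, with no change to a red value.
; Paint reads the second tag to swap the Cube's material to black, red or green and stores it in Current.
; The Boule branch only prints a debug string.
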(event `self.ReceiveBeginPlay`
  (bind _base (`self.Base`))
  (`PrimitiveComponent.SetMaterial` (`self.Cube`) 0 _base)
  (set `self.Current` _base))

(event `self.ReceiveActorBeginOverlap`
  (params (OtherActor :type "Actor Object Reference"))
  (switch `name` (`|GetArrayItem` (`Actor.Tags` OtherActor))
    (:`Boule`
      (`self.CheckIfBoule` OtherActor))
    (:`Gold`
      (`self.CheckIfGold` OtherActor))
    (:`Paint`
      (`self.CheckIfPaint` OtherActor))))

(fn `CheckIfBoule`
  (params (Actor :type "Actor Object Reference"))
  (`KismetSystemLibrary.PrintString` "Boule"))

(fn `CheckIfGold`
  (params (Actor :type "Actor Object Reference"))
  (set `self.BaseValue` (+ (`self.BaseValue`) (`self.GoldIncrease`)))
  (set `self.BlackValue` (+ (`self.BlackValue`) (`self.GoldIncrease`)))
  (set `self.GreenValue` (+ (`self.GreenValue`) (`self.GoldIncrease`)))
  (`KismetSystemLibrary.PrintString` "Gold"))

(fn `CheckIfPaint`
  (params (Actor :type "Actor Object Reference"))
  (bind _greencolor (`self.GreenColor`))
  (bind _redcolor (`self.RedColor`))
  (bind _blackcolor (`self.BlackColor`))
  (bind _output (`|GetArrayItem` (`Actor.Tags` Actor) 1))
  (switch `name` _output
    (:`Black`
      (`PrimitiveComponent.SetMaterial` (`self.Cube`) 0 _blackcolor)
      (set `self.Current` _blackcolor))
    (:`Red`
      (`PrimitiveComponent.SetMaterial` (`self.Cube`) 0 _redcolor)
      (set `self.Current` _redcolor))
    (:`Green`
      (`PrimitiveComponent.SetMaterial` (`self.Cube`) 0 _greencolor)
      (set `self.Current` _greencolor)))
  (`KismetSystemLibrary.PrintString` (`KismetStringLibrary.Concat_StrStr` "Paint: " (`KismetStringLibrary.Conv_NameToString` _output))))

(fn `UserConstructionScript`)