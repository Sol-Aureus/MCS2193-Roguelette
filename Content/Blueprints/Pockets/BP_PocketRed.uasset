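; BP_PocketRed is a pocket Blueprint that reacts to overlapping actors based on their first tag: Boule, Gold or Paint.
; Its overlap event passes the actor to a matching check function.
; Only the Gold check changes state, raising the base, black and green values by the gold increase.
; The Boule and Paint checks only print their tag name, and the Gold check prints too.
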(event `self.ReceiveActorBeginOverlap`
  (params (OtherActor :type "Actor Object Reference"))
  (switch `name` (`|GetArrayItem` (`Actor.Tags` OtherActor))
    (:`Boule`
      (`self.CheckIfBoule` OtherActor))
    (:`Gold`
      (`self.CheckIfGold` OtherActor))
    (:`Paint`
      (`self.CheckIfPaint` OtherActor))))

(fn `CheckIfBoule`
  (params (Actor :type "Object Object Reference"))
  (`KismetSystemLibrary.PrintString` "Boule"))

(fn `CheckIfGold`
  (params (Actor :type "Object Object Reference"))
  (set `self.BaseValue` (+ (`self.BaseValue`) (`self.GoldIncrease`)))
  (set `self.BlackValue` (+ (`self.BlackValue`) (`self.GoldIncrease`)))
  (set `self.GreenValue` (+ (`self.GreenValue`) (`self.GoldIncrease`)))
  (`KismetSystemLibrary.PrintString` "Gold"))

(fn `CheckIfPaint`
  (params (Actor :type "Object Object Reference"))
  (`KismetSystemLibrary.PrintString` "Paint"))

(fn `UserConstructionScript`)